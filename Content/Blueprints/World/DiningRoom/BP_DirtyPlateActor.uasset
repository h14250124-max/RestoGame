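; Dirty plate actor in the dining room that the player cleans by holding interact, after which its table is marked clean.
; Interacting while it is the character's CleaningTarget starts a looping timer that counts down only while the character's Hold flag is set.
; Each step updates a progress widget, which Tick turns toward the camera.
; At zero it sets the table's IsCleaned and destroys itself.
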(event `/Game/ThirdPerson/Blueprints/BPI_Interactable.Interactable`
  (params (Player :type "/Game/ThirdPerson/Blueprints/BP_ThirdPersonCharacter Object Reference"))
  (bind _asbp_third_person_character (cast `/Game/ThirdPerson/Blueprints/BP_ThirdPersonCharacter` (`GameplayStatics.GetPlayerCharacter` 0)))
  (if (== (`/Game/ThirdPerson/Blueprints/BP_ThirdPersonCharacter.CleaningTarget` _asbp_third_person_character) self)
    (`self.Start cleaning`)))

(event `Start cleaning`
  (bind _asbp_third_person_character (cast `/Game/ThirdPerson/Blueprints/BP_ThirdPersonCharacter` (`GameplayStatics.GetPlayerCharacter` 0)))
  (`/Engine/EditorBlueprintResources/StandardMacros.IsValid` (`/Game/ThirdPerson/Blueprints/BP_ThirdPersonCharacter.CleaningTarget` _asbp_third_person_character)
    (:`Is Valid`
      (bind _aswb_progress_timer (cast `/Game/UI/WB_ProgressTimer` (`WidgetComponent.GetWidget` (`self.CleanTimer`))))
      (set `self.WB_CleanTimer` _aswb_progress_timer)
      (bind _returnvalue (`KismetSystemLibrary.K2_SetTimerDelegate` (delegate `UpdateClean`) (`self.CleaningTimer`) true))
      (set `self.CleaningHandleTimer` _returnvalue))))

(event `UpdateClean`
  (if (`/Game/ThirdPerson/Blueprints/BP_ThirdPersonCharacter.Hold` (stale `Start cleaning` _asbp_third_person_character))
    (bind _output_get (set `self.CurrentTime` (- (`self.CurrentTime`) (`self.CleaningTimer`))))
    (`/Game/UI/WB_ProgressTimer.Update Timer` (`self.WB_CleanTimer`) _output_get (`self.MaxTimer`))
    (`KismetSystemLibrary.PrintString` "IsClean")
    (if (<= (`self.CurrentTime`) 0.0)
      (set `/Game/Blueprints/World/DiningRoom/BP_Table.IsCleaned?` true (`self.BP_Table`))
      (`self.K2_DestroyActor`))))

(event `self.ReceiveTick`
  (params (DeltaSeconds :type "Float (single-precision)"))
  (`SceneComponent.K2_SetWorldRotation` (`self.CleanTimer`) (`KismetMathLibrary.FindLookAtRotation` (`SceneComponent.K2_GetComponentLocation` (`self.CleanTimer`)) (`SceneComponent.K2_GetComponentLocation` (`PlayerCameraManager.TransformComponent` (`GameplayStatics.GetPlayerCameraManager` 0)))) false false))

(fn `NewFunction`)

(fn `UserConstructionScript`)
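; BP_PickUpWindow is a kitchen pick-up window where the player places waiting NPCs and hands over their orders.
; When unoccupied, interacting assigns the player's selected NPC and teleports it to the StandPoint.
; When occupied, it compares the held BP_Food's menu to CurrentOrder and calls OrderComplete on a match.
; Seating, order completion and NPC removal events only forward to the parent class.
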(event `/Game/ThirdPerson/Blueprints/BPI_Interactable.Interactable`
  (params (Player :type "/Game/ThirdPerson/Blueprints/BP_ThirdPersonCharacter Object Reference"))
  (bind _heldingredientactor (`/Game/ThirdPerson/Blueprints/BP_ThirdPersonCharacter.HeldIngredientActor` Player))
  (bind _selectednpc (`/Game/ThirdPerson/Blueprints/BP_ThirdPersonCharacter.SelectedNPC` Player))
  (if (`self.IsOccupied?`)
    (if (`KismetSystemLibrary.IsValid` _heldingredientactor)
      (bind _asbp_food (cast `/Game/Blueprints/World/Kitchen/BP_Food` _heldingredientactor))
      (bind _ecurrentfood (`/Game/Blueprints/World/Kitchen/BP_Food.GetMenu` _asbp_food))
      (if (`|EnumEquality` _ecurrentfood (`self.CurrentOrder`))
        (`self.Order Complete` null)))
    (else
      (`/Engine/EditorBlueprintResources/StandardMacros.IsValid` _selectednpc
        (:`Is Valid`
          (bind _output_get (set `self.AssignedNPC` _selectednpc))
          (`self.K2_SetActorLocation` _output_get (`SceneComponent.K2_GetComponentLocation` (`self.StandPoint`)) false true))))))

(event `self.The NPC Sits`
  (`parent.The NPC Sits`))

(event `self.Order Complete`
  (params (Player :type "/Game/ThirdPerson/Blueprints/BP_ThirdPersonCharacter Object Reference"))
  (`parent.Order Complete` null))

(event `self.Remove NPC`
  (`parent.Remove NPC`))

(fn `UserConstructionScript`
  (`parent.UserConstructionScript`))
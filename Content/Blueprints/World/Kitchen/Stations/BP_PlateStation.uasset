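; Kitchen plate station, derived from a parent station, that turns an ingredient into plated food.
; Its ProcessIngredient override destroys the held ingredient reference, spawns BP_Food at PlateSlot and reopens interaction.
; The Interactable event is empty; unconnected logic would accept a cuttable ingredient in a specific state and start the progress timer.
; That logic's pickup branch attaches the destroyed ingredient reference, though it assigns PlatedFood to the player.
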(event `/Game/UI/BPI/BPI_Interactable.Interactable`
  (params (Player :type "/Game/ThirdPerson/Blueprints/BP_ThirdPersonCharacter Object Reference")))

(fn `Process Ingredient`
  (`parent.Process Ingredient`)
  (`self.K2_DestroyActor` (`self.IngredientStationRef`))
  (bind _returnvalue (`|SpawnActorFromClass` "/Game/Blueprints/World/Kitchen/BP_Food.BP_Food_C" (`KismetMathLibrary.MakeTransform` (`SceneComponent.K2_GetComponentLocation` (`self.PlateSlot`))) "Undefined" "MultiplyWithRoot" null "NewEnumerator0" "NewEnumerator2" null))
  (set `self.PlatedFood` _returnvalue)
  (set `self.HasProcessFinished` true)
  (set `self.CanInteract` true))

(fn `UserConstructionScript`
  (`parent.UserConstructionScript`))
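; BP_CuttingBoard is an interactable kitchen station that takes a held ingredient for timed cutting.
; It accepts ingredients in the first enum state that implement BPI_Cutable, moves them to CuttingSlot, locks interaction and starts a progress-bar timer.
; An empty-handed player retrieves the finished ingredient onto their ChestHoldPoint.
; Progress and completion logic is not in this graph, which also holds unconnected leftover slot-and-timer nodes.
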(event `DestroyIngredient`
  (`self.K2_DestroyActor` (`self.Slot Ingredient`))
  (set `self.Slot Ingredient` null))

(event `SetIngredeintSlot`)

(event `/Game/UI/BPI/BPI_Interactable.Interactable`
  (params (Player :type "/Game/ThirdPerson/Blueprints/BP_ThirdPersonCharacter Object Reference"))
  (bind _ingredientstationref (`self.IngredientStationRef`))
  (if (`self.CanInteract`)
    (`/Engine/EditorBlueprintResources/StandardMacros.IsValid` (`/Game/ThirdPerson/Blueprints/BP_ThirdPersonCharacter.HeldIngredientActor` Player)
      (:`Is Valid`
        (bind _asbp_ingredient (cast `/Game/Blueprints/World/Kitchen/BP_Ingredient` (`/Game/ThirdPerson/Blueprints/BP_ThirdPersonCharacter.HeldIngredientActor` Player)))
        (set `self.IngredientStationRef` _asbp_ingredient)
        (bind _successful (`self.MoveIngredientFromPlayerToStationSlot` Player (`self.CuttingSlot`) (and (`|EnumEquality` (`/Game/Blueprints/World/Kitchen/BP_Ingredient.IngredientState` (`self.IngredientStationRef`)) "NewEnumerator0") (`KismetSystemLibrary.DoesImplementInterface` (`self.IngredientStationRef`) "/Game/UI/BPI/BPI_Cutable.BPI_Cutable_C"))))
        (if _successful
          (set `/Game/ThirdPerson/Blueprints/BP_ThirdPersonCharacter.HeldIngredientActor` null Player)
          (set `self.ProcessTime` 5.0)
          (set `self.ProcessSpeed` 1.0)
          (set `self.CanInteract` false)
          (`self.StartProgressBarTimer`)))
      (:`Is Not Valid`
        (if (`self.HasProcessFinished`)
          (bind _returnvalue (`self.K2_AttachToComponent` (`self.IngredientStationRef`) (`/Game/ThirdPerson/Blueprints/BP_ThirdPersonCharacter.ChestHoldPoint` Player) "None" "SnapToTarget" "KeepRelative" "KeepWorld" true))
          (if _returnvalue
            (`KismetSystemLibrary.PrintString` (`KismetStringLibrary.Concat_StrStr` (`KismetSystemLibrary.GetDisplayName` _ingredientstationref) "is" (`|GetEnumeratorNameAsString` (`/Game/Blueprints/World/Kitchen/BP_Ingredient.IngredientState` _ingredientstationref))))
            (set `/Game/ThirdPerson/Blueprints/BP_ThirdPersonCharacter.HeldIngredientActor` (`self.IngredientStationRef`) Player)
            (set `self.IngredientStationRef` null)
            (set `self.HasProcessFinished` false)))))))

(fn `UserConstructionScript`
  (`parent.UserConstructionScript`))
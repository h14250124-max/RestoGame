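; BP_Food is a kitchen food actor that the player can pick up and carry.
; On pickup it disables its collision, snaps to the player's ChestHoldPoint keeping world scale, and registers itself as the player's HeldIngredientActor.
; Getters expose its menu and item category from variables, while ingredient type, item type and prepared food queries return fixed first-enumerator values.
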(event `/Game/ThirdPerson/Blueprints/BPI_Carriable.OnPickedUp`
  (params (Player :type "/Game/ThirdPerson/Blueprints/BP_ThirdPersonCharacter Object Reference"))
  (`self.SetActorEnableCollision` false)
  (`self.K2_AttachToComponent` (`/Game/ThirdPerson/Blueprints/BP_ThirdPersonCharacter.ChestHoldPoint` Player) "None" "SnapToTarget" "SnapToTarget" "KeepWorld" false)
  (set `/Game/ThirdPerson/Blueprints/BP_ThirdPersonCharacter.HeldIngredientActor` self Player))

(fn `GetEItemCategory`
  (returns (EItem :type "/Game/UI/EItemCategory Enum"))
  (return (`self.EItem`)))

(fn `GetIngredientType`
  (returns (IngredientType :type "/Game/UI/EIngredient Enum"))
  (return "NewEnumerator0"))

(fn `GetItemType`
  (returns (EItemCategory :type "/Game/UI/EItemCategory Enum"))
  (return "NewEnumerator0"))

(fn `GetMenu`
  (returns (ECurrentFood :type "/Game/UI/EMenu Enum"))
  (return (`self.ECurrentFood`)))

(fn `GetPreparedFood`
  (returns (PreparedFood :type "/Game/UI/EPreparedFood Enum"))
  (return "NewEnumerator0"))

(fn `UserConstructionScript`)
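; BP_IngredientBoxManager is a kitchen manager that unlocks ingredient boxes one at a time, in array order.
; Each UnlockedBox event calls Unlocked on the IngredientBoxes entry at UnlockedIndex, then increments the index.
; A bounds check makes further calls do nothing once the index passes the last box.
; It has no other active logic, so progression depends entirely on that event being called.
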(event `Unlocked Box`
  (if (not (>= (`self.UnlockedIndex`) (`KismetArrayLibrary.Array_Length` (`self.IngredientBoxes`))))
    (`/Game/Blueprints/World/Kitchen/BP_IngredientBox1.Unlocked` (`|GetArrayItem` (`self.IngredientBoxes`) (`self.UnlockedIndex`)))
    (set `self.UnlockedIndex` (+ (`self.UnlockedIndex`) 1))))

(fn `UserConstructionScript`)
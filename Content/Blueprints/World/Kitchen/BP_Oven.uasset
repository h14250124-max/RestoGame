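; BP_Oven is a kitchen interactable that cooks the player's held Prepared Food into the matching BP_Food menu item.
; Interacting records the prep type, destroys the held ingredient, shows the progress widget and starts a looping timer.
; UpdateTimer counts down by CookTime, which also serves as the timer interval, and updates the widget.
; At zero it resets, spawns the food and attaches it directly to the player's chest hold point.
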(event `/Game/ThirdPerson/Blueprints/BPI_Interactable.Interactable`
  (params (Player :type "/Game/ThirdPerson/Blueprints/BP_ThirdPersonCharacter Object Reference"))
  (bind _heldingredientactor (`/Game/ThirdPerson/Blueprints/BP_ThirdPersonCharacter.HeldIngredientActor` Player))
  (bind _eitemcategory (message `/Game/ThirdPerson/Blueprints/BPI_Carriable.GetItemType` _heldingredientactor))
  (switch `/Game/UI/EItemCategory` _eitemcategory
    (:`NewEnumerator1`
      (bind _preparedfood (message `/Game/ThirdPerson/Blueprints/BPI_Carriable.GetPreparedFood` _heldingredientactor))
      (bind _output_get (set `self.E PreparedFood` _preparedfood))
      (switch `/Game/UI/EPreparedFood` _output_get
        (:`NewEnumerator0`
          _)
        (:`NewEnumerator1`
          _)
        (:`NewEnumerator2`
          _)
        (:`NewEnumerator3`
          _)
        (:`NewEnumerator5`
          _))
      (`/Engine/EditorBlueprintResources/StandardMacros.IsValid` _heldingredientactor
        (:`Is Valid`
          (`self.K2_DestroyActor` _heldingredientactor)
          (set `/Game/ThirdPerson/Blueprints/BP_ThirdPersonCharacter.HeldIngredientActor` null Player)
          (`SceneComponent.SetVisibility` (`self.CookTimer`) true false)
          (bind _aswb_progress_timer (cast `/Game/UI/WB_ProgressTimer` (`WidgetComponent.GetWidget` (`self.CookTimer`))))
          (set `self.WB_CookTimer` _aswb_progress_timer)
          (bind _returnvalue (`KismetSystemLibrary.K2_SetTimerDelegate` (delegate `UpdateTimer`) (`self.CookTime`) true)))))))

(event `UpdateTimer`
  (bind _output_get (set `self.CurrentTime` (- (`self.CurrentTime`) (`self.CookTime`))))
  (`/Game/UI/WB_ProgressTimer.Update Timer` (`self.WB_CookTimer`) _output_get (`self.MaxTime`))
  (if (<= (`self.CurrentTime`) 0.0)
    (`SceneComponent.SetVisibility` (`self.CookTimer`) false false)
    (`KismetSystemLibrary.K2_ClearAndInvalidateTimerHandle` (stale `/Game/ThirdPerson/Blueprints/BPI_Interactable.Interactable` _returnvalue))
    (set `self.CurrentTime` (`self.MaxTime`))
    (bind _returnvalue (`|SpawnActorFromClass` "/Game/Blueprints/World/Kitchen/BP_Food.BP_Food_C" (`KismetMathLibrary.Conv_VectorToTransform` (`SceneComponent.K2_GetComponentLocation` (`self.Oven`))) "Undefined" "MultiplyWithRoot" null (select `/Game/UI/EPreparedFood` (`self.E PreparedFood`) :`NewEnumerator0` "NewEnumerator0" :`NewEnumerator1` "NewEnumerator1" :`NewEnumerator2` "NewEnumerator2" :`NewEnumerator3` "NewEnumerator3" :`NewEnumerator5` "NewEnumerator4" :!type "/Game/UI/EMenu Enum") "NewEnumerator2" null))
    (bind _output_get_2 (set `/Game/ThirdPerson/Blueprints/BP_ThirdPersonCharacter.HeldIngredientActor` _returnvalue (stale `/Game/ThirdPerson/Blueprints/BPI_Interactable.Interactable` Player)))
    (`self.K2_AttachToComponent` _output_get_2 (`/Game/ThirdPerson/Blueprints/BP_ThirdPersonCharacter.ChestHoldPoint` (stale `/Game/ThirdPerson/Blueprints/BPI_Interactable.Interactable` Player)) "None" "SnapToTarget" "KeepRelative" "KeepWorld" true)))

(fn `UserConstructionScript`)
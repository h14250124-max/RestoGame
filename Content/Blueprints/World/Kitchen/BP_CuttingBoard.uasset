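; Kitchen cutting board actor that takes the ingredient the player is holding when they interact with it.
; Interactable checks the held item's type through an interface-style message, snaps ingredients to the CuttingSlot component, records their type, clears the player's hand and calls StartTimer.
; StartTimer is not defined in this graph.
; A separate DestroyIngredient event destroys the slotted ingredient and clears both references.
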(event `DestroyIngredient`
  (`self.K2_DestroyActor` (`self.Slot Ingredient`))
  (set `self.Slot Ingredient` null)
  (set `/Game/ThirdPerson/Blueprints/BP_ThirdPersonCharacter.HeldIngredientActor` null (stale `/Game/ThirdPerson/Blueprints/BPI_Interactable.Interactable` Player)))

(event `SetIngredeintSlot`
  (bind _ingredienttype (message `/Game/ThirdPerson/Blueprints/BPI_Carriable.GetIngredientType` (`/Game/ThirdPerson/Blueprints/BP_ThirdPersonCharacter.HeldIngredientActor` (stale `/Game/ThirdPerson/Blueprints/BPI_Interactable.Interactable` Player))))
  (set `self.E_Ingredient` _ingredienttype))

(event `/Game/ThirdPerson/Blueprints/BPI_Interactable.Interactable`
  (params (Player :type "/Game/ThirdPerson/Blueprints/BP_ThirdPersonCharacter Object Reference"))
  (bind _heldingredientactor (`/Game/ThirdPerson/Blueprints/BP_ThirdPersonCharacter.HeldIngredientActor` Player))
  (`KismetSystemLibrary.PrintString` "Work")
  (bind _eitemcategory (message `/Game/ThirdPerson/Blueprints/BPI_Carriable.GetItemType` _heldingredientactor))
  (switch `/Game/UI/EItemCategory` _eitemcategory
    (:`NewEnumerator0`
      (`/Engine/EditorBlueprintResources/StandardMacros.IsValid` _heldingredientactor
        (:`Is Valid`
          (bind _output_get (set `self.Slot Ingredient` _heldingredientactor))
          (`self.K2_AttachToComponent` _output_get (`self.CuttingSlot`) "None" "SnapToTarget" "KeepRelative" "KeepWorld" true)
          (`self.SetIngredeintSlot`)
          (set `/Game/ThirdPerson/Blueprints/BP_ThirdPersonCharacter.HeldIngredientActor` null Player)
          (`self.Start Timer`))))))

(fn `UserConstructionScript`
  (`parent.UserConstructionScript`))
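; Kitchen ingredient box that dispenses a BP_Ingredient when its Interactable event fires.
; The event always spawns the ingredient at SpawnPoint's transform, copies IngredientToSpawn into its type and hard-codes its mesh to Raw_steak.
; A separate SpawnIngredient function, not called within this graph, spawns at the point's location only and sets the type without changing the mesh.
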(event `self.Interactable`
  (params (Player :type "/Game/ThirdPerson/Blueprints/BP_ThirdPersonCharacter Object Reference"))
  (bind _returnvalue (`|SpawnActorFromClass` "/Game/Blueprints/World/Kitchen/BP_Ingredient.BP_Ingredient_C" (`SceneComponent.K2_GetComponentToWorld` (`self.SpawnPoint`)) "AlwaysSpawn" "MultiplyWithRoot" null null))
  (set `/Game/Blueprints/World/Kitchen/BP_Ingredient.IngredientType` (`self.IngredientToSpawn`) _returnvalue)
  (`StaticMeshComponent.SetStaticMesh` (`/Game/Blueprints/World/Kitchen/BP_Ingredient.StaticMesh` _returnvalue) "/Game/StaticMeshs/Raw_steak/StaticMeshes/Raw_steak.Raw_steak"))

(fn `SpawnIngredient`
  (bind _returnvalue (`|SpawnActorFromClass` "/Game/Blueprints/World/Kitchen/BP_Ingredient.BP_Ingredient_C" (`KismetMathLibrary.Conv_VectorToTransform` (`SceneComponent.K2_GetComponentLocation` (`self.SpawnPoint`))) "Undefined" "MultiplyWithRoot" null null))
  (set `/Game/Blueprints/World/Kitchen/BP_Ingredient.IngredientType` (`self.IngredientToSpawn`) _returnvalue))

(fn `UserConstructionScript`)
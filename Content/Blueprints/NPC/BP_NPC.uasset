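; Customer NPC for an order-and-table service game, set up at BeginPlay from a random DT_NPC row.
; Customer type adds behavior: Rowdy overwrites nearby NPCs' timer step, VIP swaps mesh, Courier sends a random order to the player's menu.
; Looping timers drive a camera-facing patience bar, first queued, then seated; queue expiry destroys the NPC.
; FinishOrder pays on success, frees the table and destroys the NPC; seated timeout counts as failure.
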(event `CourierThing`
  (if (== (`KismetMathLibrary.RandomIntegerInRange` 0 1) 0)
    (bind _output_get (set `self.Menu` "NewEnumerator0"))
    (set `self.CourierOrderString` (`|GetEnumeratorNameAsString` _output_get))
    (else
      (bind _output_get_2 (set `self.Menu` "NewEnumerator1"))
      (set `self.CourierOrderString` (`|GetEnumeratorNameAsString` _output_get_2))))
  (bind _asbp_third_person_player_controller (cast `/Game/ThirdPerson/Blueprints/BP_ThirdPersonPlayerController` (`GameplayStatics.GetPlayerController` 0)))
  (`/Game/UI/WB_OrderUI.NotifyOrderCreated` (`/Game/ThirdPerson/Blueprints/BP_ThirdPersonPlayerController.Menu Choice` _asbp_third_person_player_controller) 0 (`self.Menu`) (`self.CourierOrderString`) self))

(event `self.ReceiveBeginPlay`
  (bind _outrownames (`DataTableFunctionLibrary.GetDataTableRowNames` "/Game/ThirdPerson/Blueprints/DT_NPC.DT_NPC"))
  (bind _output_get (set `self.RowName` (`KismetArrayLibrary.Array_Random` _outrownames)))
  (bind _returnvalue (`|GetDataTableRow` "/Game/ThirdPerson/Blueprints/DT_NPC.DT_NPC" _output_get)
    (:`then`
      (bind _output_get_2 (set `self.NPC_Data` _returnvalue))
      (bind (_usestable _reward _patience _customertype) (break `/Game/ThirdPerson/Blueprints/S_NPCData` _output_get_2))
      (set `self.Reward` _reward)
      (bind _output_get_3 (set `self.Patience` _patience))
      (set `self.MaxTimer` _output_get_3)
      (set `self.new curent time` _output_get_3)
      (set `self.UsesTable` _usestable)
      (switch `/Game/ThirdPerson/Blueprints/E_CustomerType` _customertype
        (:`NewEnumerator0`
          (`self.AddTimer`))
        (:`NewEnumerator1`
          (`self.AddTimer`)
          (`KismetSystemLibrary.PrintString` "Hi i'm rowdy!!!!")
          (for _array_element (`PrimitiveComponent.GetOverlappingActors` (`self.Sphere`) "BP_NPC_C")
            (if (!= _array_element self)
              (bind _asbp_npc (cast `/Game/Blueprints/NPC/BP_NPC` _array_element))
              (`self.SpeedUpTimerRowdy`))))
        (:`NewEnumerator2`
          (`SkeletalMeshComponent.SetSkeletalMeshAsset` (`self.Mesh`) "/Game/Characters/Mannequins/Meshes/SKM_Manny_Simple.SKM_Manny_Simple")
          (`self.AddTimer`))
        (:`NewEnumerator3`
          (`self.AddTimer`)
          (`KismetSystemLibrary.PrintString` "Courier here")
          (`self.CourierThing`))))))

(event `SpeedUpTimerRowdy`
  (set `/Game/Blueprints/NPC/BP_NPC.Time` 0.04 (stale `self.ReceiveBeginPlay` _asbp_npc)))

(event `AddTimer`
  (bind _spawner (`self.Spawner`))
  (bind _aswb_progress_timer (cast `/Game/UI/WB_ProgressTimer` (`WidgetComponent.GetWidget` (`self.TimerWidget`))))
  (set `self.As WB Progress Timer` _aswb_progress_timer)
  (bind _returnvalue (`KismetSystemLibrary.K2_SetTimerDelegate` (delegate `UpdateTimer`) (`self.Time`) true))
  (set `self.Queue Timer` _returnvalue)
  (`/Engine/EditorBlueprintResources/StandardMacros.IsValid` _spawner
    (:`Is Valid`
      (`/Game/Blueprints/NPC/BP_NPCSpawner.UnregisterNPC` _spawner self))))

(event `UpdateTimer`
  (bind _output_get (set `self.CurrentTimer` (- (`self.CurrentTimer`) (`self.Time`))))
  (`/Game/UI/WB_ProgressTimer.Update Timer` (`self.As WB Progress Timer`) _output_get (`self.MaxTimer`))
  (if (<= (`self.CurrentTimer`) 0.0)
    (`self.K2_DestroyActor`)
    (bind _returnvalue (`GameplayStatics.GetActorOfClass` "/Game/Blueprints/NPC/BP_NPCSpawner.BP_NPCSpawner_C"))))

(event `self.ReceiveTick`
  (params (DeltaSeconds :type "Float (single-precision)"))
  ; 3d timer
  (`SceneComponent.K2_SetWorldRotation` (`self.TimerWidget`) (`KismetMathLibrary.FindLookAtRotation` (`SceneComponent.K2_GetComponentLocation` (`self.TimerWidget`)) (`SceneComponent.K2_GetComponentLocation` (`PlayerCameraManager.TransformComponent` (`GameplayStatics.GetPlayerCameraManager` 0)))) false false))

(event `/Game/ThirdPerson/Blueprints/BPI_Interactable.Interactable`
  (params (Player :type "/Game/ThirdPerson/Blueprints/BP_ThirdPersonCharacter Object Reference"))
  (bind _asbp_third_person_character (cast `/Game/ThirdPerson/Blueprints/BP_ThirdPersonCharacter` (`GameplayStatics.GetPlayerCharacter` 0)))
  (set `/Game/ThirdPerson/Blueprints/BP_ThirdPersonCharacter.SelectedNPC` self _asbp_third_person_character))

(event `Finish Order`
  (params (IsSucess :type Boolean) (TableId :type Integer))
  (bind _bp_table (`self.BP Table`))
  (`/Engine/EditorBlueprintResources/StandardMacros.IsValid` _bp_table
    (:`Is Valid`
      (if IsSucess
        (bind _asbp_third_person_character (cast `/Game/ThirdPerson/Blueprints/BP_ThirdPersonCharacter` (`GameplayStatics.GetPlayerCharacter` 0)))
        (bind _output_get (set `/Game/ThirdPerson/Blueprints/BP_ThirdPersonCharacter.Money` (+ (`/Game/ThirdPerson/Blueprints/BP_ThirdPersonCharacter.Money` _asbp_third_person_character) 10) _asbp_third_person_character))
        (bind _asbp_third_person_player_controller (cast `/Game/ThirdPerson/Blueprints/BP_ThirdPersonPlayerController` (`GameplayStatics.GetPlayerController` 0)))
        (`/Game/UI/WB_OrderUI.UpdateMoney` (`/Game/ThirdPerson/Blueprints/BP_ThirdPersonPlayerController.Menu Choice` _asbp_third_person_player_controller) (`KismetTextLibrary.Conv_IntToText` _output_get))
        (`KismetSystemLibrary.PrintString` (`KismetStringLibrary.Concat_StrStr` "Money: " (`KismetStringLibrary.Conv_IntToString` _output_get))))
      (`/Game/Blueprints/World/DiningRoom/BP_Table.Remove NPC` _bp_table)
      (set `self.BP Table` null)
      (`KismetSystemLibrary.PrintString` "Wny no work")
      (`self.K2_DestroyActor`)
      (`KismetSystemLibrary.K2_ClearAndInvalidateTimerHandle` (`self.Sit Timer`))
      (bind _asbp_third_person_player_controller_2 (cast `/Game/ThirdPerson/Blueprints/BP_ThirdPersonPlayerController` (`GameplayStatics.GetPlayerController` 0)))
      (message `/Game/ThirdPerson/Blueprints/BPI_TheOrderUI.NotifyOrderFinished` (`/Game/ThirdPerson/Blueprints/BP_ThirdPersonPlayerController.Menu Choice` _asbp_third_person_player_controller_2) TableId))))

(event `ClearAssignedTable`
  (set `self.AssignedTable` null))

(event `Set Table`
  (params (BP_Table :type "/Game/Blueprints/World/DiningRoom/BP_Table Object Reference"))
  (set `self.BP Table` BP_Table))

(event `Sit in table`
  (`KismetSystemLibrary.K2_ClearAndInvalidateTimerHandle` (`self.Queue Timer`))
  (`KismetSystemLibrary.K2_SetTimerDelegate` (delegate `ResetTimer`) (`self.MaxTimer`))
  (set `self.CurrentTimer` (`self.MaxTimer`))
  (bind _returnvalue (`KismetSystemLibrary.K2_SetTimerDelegate` (delegate `Set Timer`) (`self.Time`) true))
  (set `self.Sit Timer` _returnvalue))

(event `ReduceTimer`
  (bind _output_get (set `self.CurrentTimer` (- (`self.CurrentTimer`) 0.6)))
  (`/Game/UI/WB_ProgressTimer.Update Timer` (`self.As WB Progress Timer`) _output_get (`self.MaxTimer`)))

(event `Set Timer`
  (bind _output_get (set `self.CurrentTimer` (- (`self.CurrentTimer`) (`self.Time`))))
  (`/Game/UI/WB_ProgressTimer.Update Timer` (`self.As WB Progress Timer`) _output_get (`self.MaxTimer`))
  (if (<= (`self.CurrentTimer`) 0.0)
    _))

(event `ResetTimer`
  (`self.Finish Order` false (`/Game/Blueprints/World/DiningRoom/BP_Table.TableID` (`self.BP Table`))))

(event `Assign To Table`
  (params (BP_Table :type "/Game/Blueprints/World/DiningRoom/BP_Table Object Reference"))
  (bind _standpoint (`/Game/Blueprints/World/DiningRoom/BP_Table.StandPoint` BP_Table))
  (`/Engine/EditorBlueprintResources/StandardMacros.IsValid` BP_Table
    (:`Is Valid`
      (`/Engine/EditorBlueprintResources/StandardMacros.IsValid` _standpoint
        (:`Is Valid`
          (bind _output_get (set `/Game/Blueprints/World/DiningRoom/BP_Table.AssignedNPC` self BP_Table))
          (`self.K2_SetActorLocation` _output_get (`SceneComponent.K2_GetComponentLocation` _standpoint) false true))))))

(fn `UserConstructionScript`)